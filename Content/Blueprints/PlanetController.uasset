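; PlanetController manages unit selection and planet clicks, apparently as a player controller for an RTS-style game, with movement orders left unfinished.
; AddSelected toggles units in UnitsSelected and notifies each through IsSelectedMessage.
; ClickPlanet computes a near-square grid from the selection count and traces under the mouse, but its loop is empty and MovementMessage is unwired.
; A separate helper only prints an angle derived from planet size, unit size and spacing.
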(event Custom|Add%20Selected
  (params (Actor%20touched :type Actor%20Object%20Reference))
  (bind _unitsselected (Variables|Default|GetUnitsSelected))
  (if (< (Utilities|Array|FindItem _unitsselected Actor%20touched) 0)
    (Utilities|Array|Add _unitsselected Actor%20touched)
    (Class|AIInterface|IsSelected(Message) Actor%20touched true)
    (else
      (Utilities|Array|RemoveItem _unitsselected Actor%20touched)
      (Class|AIInterface|IsSelected(Message) Actor%20touched false))))

(event Custom|ClickPlanet
  (bind (_worldlocation _worlddirection) (Game|Player|ConvertMouseLocationToWorldSpace))
  (bind _unitsselected (Variables|Default|GetUnitsSelected))
  (CallFunction|ChooseNumberOfLine (Utilities|Array|Length _unitsselected))
  (bind _outhit (Collision|LineTraceByChannel _worldlocation (+ _worldlocation (* _worlddirection 1e+04)) "TraceTypeQuery1" false 0 "ForDuration"))
  (Variables|Default|SetImpact%20Point (.ImpactPoint (Collision|BreakHitResult _outhit)))
  (for _array_element _unitsselected
    _))

(event EventBeginPlay)

(event EventTick
  (params (DeltaSeconds :type Float%20%28single-precision%29)))

(fn ConstructionScript)

(fn ChooseNumberOfLine
  (params (Length :type Integer))
  (bind _returnvalue (Math|Conversions|ToFloat(Integer) Length))
  (bind _returnvalue_2 (Math|Conversions|ToFloat(Integer) Length))
  (bind _returnvalue_3 (Math|Float|Sqrt _returnvalue))
  (bind _returnvalue_4 (Math|Float|Ceil _returnvalue_3))
  (bind _returnvalue_5 (Math|Conversions|ToFloat(Integer) _returnvalue_4))
  (bind (_remainder _returnvalue_6) (Math|Float|Division(WholeandRemainder) _returnvalue_2 _returnvalue_5))
  (bind _returnvalue_7 (Math|Float|Round _remainder))
  (return _returnvalue_4 (+ (Math|Integer|Clamp(Integer) (Math|Float|Truncate _remainder) 0 1) _returnvalue_6) (Math|Integer|SelectInt _returnvalue_7 _returnvalue_4 (Math|Conversions|ToBoolean(Integer) _returnvalue_7))))

(fn CalculateAnglefromPlanetandUnitSize
  (params (PlanetSize :type Float%20%28single-precision%29) (Espacement :type Float%20%28single-precision%29) (Unit%20Size :type Float%20%28single-precision%29))
  (Development|PrintString (Utilities|String|ToString(Float) (Class|KismetMathLibrary|DegAtan2 PlanetSize (+ Espacement Unit%20Size)))))