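; Clickable mine on a planet that earns minerals for the game mode while miner units work it.
; Clicking its components sets the PlanetController's impact point and moves all units there.
; A miner entering the box starts a looping timer that adds progress per overlapping miner, awards minerals when full and stops when no units remain.
; BeginPlay traces four arrows toward the planet, caching points from which CollisionFromHere picks using dot-product and distance tests.
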(event OnClicked(w1)
  (params (TouchedComponent :type Primitive%20Component%20Object%20Reference) (ButtonPressed :type Key%20Structure))
  (bind _asplanet_controller (Utilities|Casting|CastToPlanetController (Game|GetPlayerController 0)))
  (Variables|/Game/Blueprints/PlanetController.PlanetController_C|SetImpact%20Point _asplanet_controller (Transformation|GetWorldLocation (Variables|Default|GetArrow)))
  (Default|MoveAllUnits _asplanet_controller))

(event OnClicked(Cube)
  (params (TouchedComponent :type Primitive%20Component%20Object%20Reference) (ButtonPressed :type Key%20Structure))
  (bind _asplanet_controller (Utilities|Casting|CastToPlanetController (Game|GetPlayerController 0)))
  (Variables|/Game/Blueprints/PlanetController.PlanetController_C|SetImpact%20Point _asplanet_controller (Transformation|GetWorldLocation (Variables|Default|GetArrow)))
  (Default|MoveAllUnits _asplanet_controller))

(event OnClicked(Box)
  (params (TouchedComponent :type Primitive%20Component%20Object%20Reference) (ButtonPressed :type Key%20Structure))
  (bind _asplanet_controller (Utilities|Casting|CastToPlanetController (Game|GetPlayerController 0)))
  (Variables|/Game/Blueprints/PlanetController.PlanetController_C|SetImpact%20Point _asplanet_controller (Transformation|GetWorldLocation (Variables|Default|GetArrow)))
  (Default|MoveAllUnits _asplanet_controller))

(event OnClicked(w)
  (params (TouchedComponent :type Primitive%20Component%20Object%20Reference) (ButtonPressed :type Key%20Structure))
  (bind _asplanet_controller (Utilities|Casting|CastToPlanetController (Game|GetPlayerController 0)))
  (Variables|/Game/Blueprints/PlanetController.PlanetController_C|SetImpact%20Point _asplanet_controller (Transformation|GetWorldLocation (Variables|Default|GetArrow)))
  (Default|MoveAllUnits _asplanet_controller))

(event OnComponentBeginOverlap(Box)
  (params (OverlappedComponent :type Primitive%20Component%20Object%20Reference) (OtherActor :type Actor%20Object%20Reference) (OtherComp :type Primitive%20Component%20Object%20Reference) (OtherBodyIndex :type Integer) (bFromSweep :type Boolean) (SweepResult :type Hit%20Result%20Structure%20%28by%20ref%29))
  (if (Utilities|DoesObjectImplementInterface OtherActor "/Game/Blueprints/AI/AI_Miners.AI_Miners_C")
    (if (not (Variables|Default|GetActuallyMining))
      (CallFunction|StartMining))
    (elif (Utilities|DoesObjectImplementInterface OtherActor "/Game/Blueprints/AI/AI_Interface.AI_Interface_C")
      (Development|PrintString "Not a miner" true true "(R=1.000000,G=0.000000,B=0.029075,A=1.000000)"))))

(event Custom|StartMining
  (Variables|Default|SetActuallyMining true)
  (Utilities|Time|SetTimerbyEvent (delegate Custom|Mining) 1.0 true)
  (Development|PrintString "StartMining"))

(event Custom|Mining
  (bind _box (Variables|Default|GetBox))
  (bind _overlappingactors (Collision|GetOverlappingActors _box "/Game/Blueprints/AI/UnitPawn.UnitPawn_C" :!class /Script/Engine.PrimitiveComponent))
  (if (Math|Conversions|ToBoolean(Integer) (Utilities|Array|Length _overlappingactors))
    (for _array_element _overlappingactors
      (if (Utilities|DoesObjectImplementInterface _array_element "/Game/Blueprints/AI/AI_Miners.AI_Miners_C")
        (Variables|Default|SetPercentMining (+ (Variables|Default|GetPercentMining) 5.0))))
    ;[1 1 1] Check Mining State
    (if (>= (Variables|Default|GetPercentMining) 1e+02)
      (Variables|Default|SetPercentMining 0.0)
      (bind _asplanet_game_mode (Utilities|Casting|CastToPlanetGameMode (Game|GetGameMode)))
      (Default|IncreaseMinerai _asplanet_game_mode (Variables|Default|GetMineValueIncrease)))
    (else
      (Variables|Default|SetActuallyMining false)
      (Utilities|Time|SetTimerbyEvent (delegate Custom|Mining) 0.0))))

(event EventBeginPlay
  (bind _outhit (Collision|LineTraceByChannel (Transformation|GetWorldLocation (Variables|Default|GetArrowDown)) (Transformation|GetActorLocation (Variables|Default|GetPlanetOwner)) "TraceTypeQuery1" false 0 "None"))
  (Variables|Default|SetDownLoc (.Location (Collision|BreakHitResult _outhit)))
  (bind _outhit_2 (Collision|LineTraceByChannel (Transformation|GetWorldLocation (Variables|Default|GetArrowUp)) (Transformation|GetActorLocation (Variables|Default|GetPlanetOwner)) "TraceTypeQuery1" false 0 "None"))
  (Variables|Default|SetUpLoc (.Location (Collision|BreakHitResult _outhit_2)))
  (bind _outhit_3 (Collision|LineTraceByChannel (Transformation|GetWorldLocation (Variables|Default|GetArrowBehind)) (Transformation|GetActorLocation (Variables|Default|GetPlanetOwner)) "TraceTypeQuery1" false 0 "None"))
  (Variables|Default|SetBehindLoc (.Location (Collision|BreakHitResult _outhit_3)))
  (bind _outhit_4 (Collision|LineTraceByChannel (Transformation|GetWorldLocation (Variables|Default|GetArrowFront)) (Transformation|GetActorLocation (Variables|Default|GetPlanetOwner)) "TraceTypeQuery1" false 0 "None"))
  (Variables|Default|SetFrontLoc (.Location (Collision|BreakHitResult _outhit_4))))

(event Collision|EventActorBeginOverlap
  (params (OtherActor :type Actor%20Object%20Reference)))

(event EventTick
  (params (DeltaSeconds :type Float%20%28single-precision%29)))

(fn ConstructionScript)

(fn CollisionfromHere
  (params (Start :type Vector :default "0, 0, 0"))
  (bind _downloc (Variables|Default|GetDownLoc))
  (bind _behindloc (Variables|Default|GetBehindLoc))
  (bind _frontloc (Variables|Default|GetFrontLoc))
  (bind _uploc (Variables|Default|GetUpLoc))
  (bind _uploc_2 (Variables|Default|GetUpLoc))
  (bind _downloc_2 (Variables|Default|GetDownLoc))
  (bind _returnvalue (Math|Vector|GetUnitDirection(Vector) _downloc _uploc))
  (bind _returnvalue_2 (Math|Vector|DotProduct Start _returnvalue))
  (Development|PrintString "BBB")
  (Development|PrintString (Utilities|String|ToString(Float) _returnvalue_2))
  (Development|PrintString (Utilities|String|ToString(Float) (Math|Vector|DotProduct Start (Math|Vector|GetUnitDirection(Vector) (Variables|Default|GetBehindLoc) (Variables|Default|GetFrontLoc)))))
  (if (Math|Float|NearlyEqual(Float) _returnvalue_2 0.0 0.1)
    (return (Math|Vector|SelectVector _uploc_2 _downloc_2 (< (Math|Vector|VectorLength (- _uploc_2 Start)) (Math|Vector|VectorLength (- _downloc_2 Start)))))
    (else
      (return (Math|Vector|SelectVector _behindloc _frontloc (< (Math|Vector|VectorLength (- _behindloc Start)) (Math|Vector|VectorLength (- _frontloc Start))))))))