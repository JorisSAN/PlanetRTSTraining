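; UnitPawn is a selectable unit pawn that moves toward a commanded goal location.
; Clicking its Box registers it with PlanetController's selection, and IsSelected swaps the cube material to show that state.
; Movement sets GoalLocation; while NeedMovement is set, Tick adds input toward it until reached.
; Tick also applies Velocity and the pending input vector directly as swept world offsets, with debug prints throughout.
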(event OnClicked(Box)
  (params (TouchedComponent :type Primitive%20Component%20Object%20Reference) (ButtonPressed :type Key%20Structure :default "None"))
  (bind _asplanet_controller (Utilities|Casting|CastToPlanetController (Game|GetPlayerController 0)))
  (Default|AddSelected _asplanet_controller self)
  (Development|PrintString "Click"))

(event OnEndCursorOver(Box)
  (params (TouchedComponent :type Primitive%20Component%20Object%20Reference))
  (Development|PrintString "UnOver"))

(event OnBeginCursorOver(Box)
  (params (TouchedComponent :type Primitive%20Component%20Object%20Reference))
  (Development|PrintString "OVer"))

(event EventBeginPlay
  (Variables|Default|SetGoalLocation (Transformation|GetActorLocation)))

(event Collision|EventActorBeginOverlap
  (params (OtherActor :type Actor%20Object%20Reference)))

(event EventTick
  (params (DeltaSeconds :type Float%20%28single-precision%29))
  (bind _returnvalue (Class|Pawn|GetPendingMovementInputVector))
  (bind _goallocation (Variables|Default|GetGoalLocation))
  (Utilities|FlowControl|Sequence
    (:then_0
      (if (not (Math|Vector|Equal(Vector) (Variables|Default|GetGoalLocation) (Transformation|GetActorLocation) 1.0))
        (if (Variables|Default|GetNeedMovement)
          ;[1 1 1] Mouvement
          (Development|PrintString (Utilities|String|ToString(Vector) _goallocation) false false)
          (Pawn|Input|AddMovementInput (Math|Vector|GetUnitDirection(Vector) (Transformation|GetActorLocation) _goallocation) 1.0 false))))
    (:then_1
      (Transformation|AddActorWorldOffset (Variables|Default|GetVelocity) true)
      (Development|PrintString (Utilities|String|ToString(Vector) _returnvalue))
      (Transformation|AddActorWorldOffset (* _returnvalue 1.0) true))))

(event EventIsSelected
  (params (Selected :type Boolean))
  (Rendering|Material|SetMaterial (Variables|Default|GetCube) 0 (select Selected "/Game/Material/Mat_AI_Selected.Mat_AI_Selected" "/Game/Material/Mat_AI.Mat_AI")))

(event EventMovement
  (params (Location :type Vector :default "0, 0, 0"))
  (Variables|Default|SetGoalLocation Location))

(fn ConstructionScript)

(fn IsGravityOn?
  (return true))