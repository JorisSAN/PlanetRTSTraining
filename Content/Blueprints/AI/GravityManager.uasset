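; Gravity manager that pulls units toward planets, caching GravityApply actors and BP_Planet actors at BeginPlay.
; Each Tick, it picks the planet with the highest Gravity-over-distance for every gravity-enabled actor.
; It moves the UnitPawn at fixed speed toward that planet's surface with up facing away, or zeroes velocity when a squared-distance sphere test passes.
; Gravity strength only affects planet choice, and the IsLand overlap check is not called here.
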(event EventBeginPlay
  (bind _outactors (Actor|GetAllActorswithInterface "/Game/Blueprints/AI/GravityApply.GravityApply_C"))
  (Variables|Default|SetActorsAffected _outactors)
  (bind _outactors_2 (Actor|GetAllActorsOfClass "/Game/Blueprints/BP_Planet.BP_Planet_C"))
  (Variables|Default|SetPlanets _outactors_2))

(event EventTick
  (params (DeltaSeconds :type Float%20%28single-precision%29))
  (for _array_element (Variables|Default|GetActorsAffected)
    (bind _gravited (Class|GravityApply|IsGravityOn?(Message) _array_element))
    (if _gravited
      (Variables|Default|SetHighestGravity 0.0)
      (Variables|Default|SetSelectedPlanet 0)
      (for _array_element_2 (Variables|Default|GetPlanets)
        (if (> (/ (Variables|/Game/Blueprints/BP_Planet.BP_Planet_C|GetGravity _array_element_2) (/ (Transformation|GetDistanceTo _array_element _array_element_2) 1e+02)) (Variables|Default|GetHighestGravity))
          (Variables|Default|SetHighestGravity (/ (Variables|/Game/Blueprints/BP_Planet.BP_Planet_C|GetGravity _array_element_2) (/ (Transformation|GetDistanceTo _array_element _array_element_2) 1e+02)))
          (Variables|Default|SetSelectedPlanet _array_element_2)))
      (bind _selectedplanet (Variables|Default|GetSelectedPlanet)
        (:then
          (bind _asunit_pawn (Utilities|Casting|CastToUnitPawn _array_element))
          (if (< (|((((Px-Cx)*(Px-Cx))+((Py-Cy)*(Py-Cy)))+((Pz-Cz)*(Pz-Cz))) (.x (+ (Transformation|GetActorLocation _array_element) (* (Math|Vector|Normalize (- (+ (Transformation|GetActorLocation _selectedplanet) (* (Math|Vector|Normalize (* (- (Transformation|GetActorLocation _selectedplanet) (Transformation|GetActorLocation _array_element)) -1.0)) (* (.x (Transformation|GetActorScale3D _selectedplanet)) 5e+01))) (Transformation|GetActorLocation _array_element))) 1e+01))) (.X (Math|Vector|BreakVector (- (Transformation|GetActorLocation _selectedplanet) (Transformation|GetActorLocation _array_element)))) (.y (+ (Transformation|GetActorLocation _array_element) (* (Math|Vector|Normalize (- (+ (Transformation|GetActorLocation _selectedplanet) (* (Math|Vector|Normalize (* (- (Transformation|GetActorLocation _selectedplanet) (Transformation|GetActorLocation _array_element)) -1.0)) (* (.x (Transformation|GetActorScale3D _selectedplanet)) 5e+01))) (Transformation|GetActorLocation _array_element))) 1e+01))) (.Y (Math|Vector|BreakVector (- (Transformation|GetActorLocation _selectedplanet) (Transformation|GetActorLocation _array_element)))) (.z (+ (Transformation|GetActorLocation _array_element) (* (Math|Vector|Normalize (- (+ (Transformation|GetActorLocation _selectedplanet) (* (Math|Vector|Normalize (* (- (Transformation|GetActorLocation _selectedplanet) (Transformation|GetActorLocation _array_element)) -1.0)) (* (.x (Transformation|GetActorScale3D _selectedplanet)) 5e+01))) (Transformation|GetActorLocation _array_element))) 1e+01))) (.Z (Math|Vector|BreakVector (- (Transformation|GetActorLocation _selectedplanet) (Transformation|GetActorLocation _array_element))))) (* (* (.x (Transformation|GetActorScale3D _selectedplanet)) 1e+02) (* (.x (Transformation|GetActorScale3D _selectedplanet)) 1e+02)))
            (Variables|/Game/Blueprints/AI/UnitPawn.UnitPawn_C|SetVelocity _asunit_pawn "0, 0, 0")
            (else
              (Variables|/Game/Blueprints/AI/UnitPawn.UnitPawn_C|SetVelocity _asunit_pawn (* (Math|Vector|Normalize (- (+ (Transformation|GetActorLocation _selectedplanet) (* (Math|Vector|Normalize (* (- (Transformation|GetActorLocation _selectedplanet) (Transformation|GetActorLocation _array_element)) -1.0)) (* (.x (Transformation|GetActorScale3D _selectedplanet)) 5e+01))) (Transformation|GetActorLocation _array_element))) 1e+01))
              (Transformation|SetActorRotation _array_element (Math|Rotator|MakeRotfromZ (* (- (Transformation|GetActorLocation _selectedplanet) (Transformation|GetActorLocation _array_element)) -1.0))))))
        (:else)))))

(fn ConstructionScript)

(fn IsLand
  (params (Unit :type Unit%20Pawn%20Object%20Reference))
  (return (not (== (Utilities|Array|Length (Collision|GetOverlappingActors (Variables|/Game/Blueprints/AI/UnitPawn.UnitPawn_C|GetBox Unit) "/Game/Blueprints/BP_Planet.BP_Planet_C" :!class /Script/Engine.PrimitiveComponent)) 0))))