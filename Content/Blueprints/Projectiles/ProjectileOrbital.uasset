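; Projectile fired along a curved ballistic arc around the nearest BP_Planet toward a preset end point.
; Launch derives horizontal velocity from surface arc length and vertical velocity from height difference, flight time and planet gravity.
; Tick realigns the actor to the planet, steps the Projectile component locally, snaps the actor to it, and destroys it below the surface.
; Overlap damage logic is disconnected, so hits have no effect.
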(event OnComponentBeginOverlap(TriggerExplosion)
  (params (OverlappedComponent :type Primitive%20Component%20Object%20Reference) (OtherActor :type Actor%20Object%20Reference) (OtherComp :type Primitive%20Component%20Object%20Reference) (OtherBodyIndex :type Integer) (bFromSweep :type Boolean) (SweepResult :type Hit%20Result%20Structure%20%28by%20ref%29))
  (if (Variables|Default|GetisLaunch)
    (if (!= OtherActor (Variables|GameDesignMissile|GetUnitOwner))
      _)))

(event Custom|Launch
  (params (owner :type Actor%20Object%20Reference))
  (bind _self self)
  (Variables|GameDesignMissile|SetUnitOwner owner)
  (bind _outactors (Actor|GetAllActorsOfClass "/Game/Blueprints/BP_Planet.BP_Planet_C"))
  (Variables|Default|SetNearestPlanet (Utilities|Array|Get(acopy) _outactors))
  (for _array_element _outactors
    (if (< (Transformation|GetDistanceTo _array_element _self) (Transformation|GetDistanceTo (Variables|Default|GetNearestPlanet) _self))
      (Variables|Default|SetNearestPlanet _array_element)))
  (Variables|Default|SetXVelocity (/ (|((APB*PP)/360) (Class|KismetMathLibrary|DegAcos (|((((a*a)+(b*b))-(c*c))/((2*a)*b)) (* (.x (Transformation|GetActorScale3D (Variables|Default|GetNearestPlanet))) 5e+01) (* (.x (Transformation|GetActorScale3D (Variables|Default|GetNearestPlanet))) 5e+01) (Math|Vector|Distance(Vector) (Transformation|GetActorLocation) (Variables|Default|GetEndPoint)))) (* 2.0 (Math|Trig|GetPI) (* (.x (Transformation|GetActorScale3D (Variables|Default|GetNearestPlanet))) 5e+01))) (* (/ (|((APB*PP)/360) (Class|KismetMathLibrary|DegAcos (|((((a*a)+(b*b))-(c*c))/((2*a)*b)) (* (.x (Transformation|GetActorScale3D (Variables|Default|GetNearestPlanet))) 5e+01) (* (.x (Transformation|GetActorScale3D (Variables|Default|GetNearestPlanet))) 5e+01) (Math|Vector|Distance(Vector) (Transformation|GetActorLocation) (Variables|Default|GetEndPoint)))) (* 2.0 (Math|Trig|GetPI) (* (.x (Transformation|GetActorScale3D (Variables|Default|GetNearestPlanet))) 5e+01))) (Variables|Default|GetDistanceMax)) (Variables|Default|GetDeltaTMax))))
  (Variables|Default|SetYVelocity (|((Dy-((0.500000*g)*(t*t)))/t) (- (Math|Vector|Distance(Vector) (Transformation|GetActorLocation (Variables|Default|GetNearestPlanet)) (Transformation|GetActorLocation)) (Math|Vector|Distance(Vector) (Variables|Default|GetEndPoint) (Transformation|GetActorLocation (Variables|Default|GetNearestPlanet)))) (Variables|/Game/Blueprints/BP_Planet.BP_Planet_C|GetGravity (Variables|Default|GetNearestPlanet)) (* (/ (|((APB*PP)/360) (Class|KismetMathLibrary|DegAcos (|((((a*a)+(b*b))-(c*c))/((2*a)*b)) (* (.x (Transformation|GetActorScale3D (Variables|Default|GetNearestPlanet))) 5e+01) (* (.x (Transformation|GetActorScale3D (Variables|Default|GetNearestPlanet))) 5e+01) (Math|Vector|Distance(Vector) (Transformation|GetActorLocation) (Variables|Default|GetEndPoint)))) (* 2.0 (Math|Trig|GetPI) (* (.x (Transformation|GetActorScale3D (Variables|Default|GetNearestPlanet))) 5e+01))) (Variables|Default|GetDistanceMax)) (Variables|Default|GetDeltaTMax))))
  (Variables|Default|SetisLaunch true))

(event EventTick
  (params (DeltaSeconds :type Float%20%28single-precision%29))
  (bind _returnvalue (Transformation|GetActorLocation))
  (bind _returnvalue_2 (Transformation|GetActorLocation))
  (bind _returnvalue_3 (Math|Trig|GetPI))
  (bind _self self)
  (bind _endpoint (Variables|Default|GetEndPoint))
  (bind _projectile (Variables|Default|GetProjectile))
  (bind _nearestplanet (Variables|Default|GetNearestPlanet))
  (bind _xvelocity (Variables|Default|GetXVelocity))
  (bind _nearestplanet_2 (Variables|Default|GetNearestPlanet))
  (bind _nearestplanet_3 (Variables|Default|GetNearestPlanet))
  (bind _nearestplanet_4 (Variables|Default|GetNearestPlanet))
  (bind _returnvalue_4 (Transformation|GetActorLocation _nearestplanet_4))
  (bind _returnvalue_5 (- _endpoint _returnvalue_2))
  (bind _returnvalue_6 (Transformation|GetActorScale3D _nearestplanet_2))
  (bind _returnvalue_7 (Transformation|GetDistanceTo _self _nearestplanet_3))
  (bind _returnvalue_8 (* _xvelocity DeltaSeconds))
  (bind _relativelocation (Variables|/Script/Engine.SceneComponent|GetRelativeLocation _projectile))
  (bind _gravity (Variables|/Game/Blueprints/BP_Planet.BP_Planet_C|GetGravity _nearestplanet))
  (bind _returnvalue_9 (- _returnvalue_4 _returnvalue))
  (bind _returnvalue_10 (* (.x _returnvalue_6) 5e+01))
  (bind _returnvalue_11 (* 2.0 _returnvalue_3 _returnvalue_10))
  (bind _returnvalue_12 (|((APB*360)/PP) _returnvalue_8 _returnvalue_11))
  (bind _returnvalue_13 (- 9e+01 _returnvalue_12))
  (bind _returnvalue_14 (Math|Trig|Tan(Degrees) _returnvalue_13))
  (bind _returnvalue_15 (/ _returnvalue_7 _returnvalue_14))
  (if (Variables|Default|GetisLaunch)
    (CallFunction|IsinEarth)
    (Transformation|SetActorRotation (Math|Rotator|MakeRotfromXZ (Math|Vector|RotateVectorAroundAxis _returnvalue_5 (- 9e+01 (Class|KismetMathLibrary|DegAcos (/ (Math|Vector|DotProduct _returnvalue_9 _returnvalue_5) (* (Math|Vector|VectorLength _returnvalue_5) (Math|Vector|VectorLength _returnvalue_9))))) (Math|Vector|CrossProduct (Math|Vector|Normalize _returnvalue_9) (Math|Vector|Normalize _returnvalue_5))) _returnvalue_9))
    (Utilities|IsValid _projectile
      (:Is%20Valid
        (Transformation|SetRelativeLocation _projectile (Math|Vector|MakeVector _returnvalue_15 0.0 (* (* (|((y0+(V0y*t))+((0.500000*g)*(t*t))) (.y _relativelocation) (* (Variables|Default|GetYVelocity) -1.0) DeltaSeconds _gravity) (/ _returnvalue_15 (|(x0+(v0x*Dt)) (.x _relativelocation) _xvelocity DeltaSeconds))) -1.0)) false false)
        (Transformation|SetActorLocation (Transformation|GetWorldLocation _projectile) false false)
        (Utilities|IsValid _projectile
          (:Is%20Valid
            (Transformation|SetRelativeLocation _projectile "0, 0, 0" false false)
            (Variables|Default|SetYVelocity (+ (Variables|Default|GetYVelocity) (* _gravity DeltaSeconds)))))))))

(fn ConstructionScript)

(fn SetEndPoint
  (params (EndPosition :type Vector))
  (Variables|Default|SetEndPoint EndPosition))

(fn IsinEarth
  (bind _nearestplanet (Variables|Default|GetNearestPlanet))
  (if (< (Transformation|GetDistanceTo _nearestplanet) (* (.x (Transformation|GetActorScale3D _nearestplanet)) 5e+01))
    (Actor|DestroyActor)))