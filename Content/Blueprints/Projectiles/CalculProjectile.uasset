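; Projectile actor that flies an arc toward the first EndPoint actor, using the gravity of the nearest BP_Planet.
; On BeginPlay it faces the target, scales flight time by distance over DistanceMax, and solves both starting velocities with kinematic equations.
; Tick moves the Projectile component by hand in local X (forward) and Y (arc), adding gravity to the Y velocity each frame.
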(event EventBeginPlay
  (bind _self self)
  (bind _outactors (Actor|GetAllActorsOfClass "/Game/Blueprints/Projectiles/EndPoint.EndPoint_C"))
  (Variables|Default|SetEndPoint (Transformation|GetActorLocation (Utilities|Array|Get(acopy) _outactors)))
  (bind _outactors_2 (Actor|GetAllActorsOfClass "/Game/Blueprints/BP_Planet.BP_Planet_C"))
  (Variables|Default|SetNearestPlanet (Utilities|Array|Get(acopy) _outactors_2))
  (for _array_element _outactors_2
    (if (< (Transformation|GetDistanceTo _array_element _self) (Transformation|GetDistanceTo (Variables|Default|GetNearestPlanet) _self))
      (Variables|Default|SetNearestPlanet _array_element)))
  (Transformation|SetActorRotation (Math|Rotator|MakeRotationfromAxes (- (Variables|Default|GetEndPoint) (Transformation|GetActorLocation)) "0, 0, 0" "0, 0, 0"))
  (Variables|Default|SetXVelocity (/ (Math|Vector|Distance(Vector) (Transformation|GetActorLocation) (Variables|Default|GetEndPoint)) (* (/ (Math|Vector|Distance(Vector) (Transformation|GetActorLocation) (Variables|Default|GetEndPoint)) (Variables|Default|GetDistanceMax)) (Variables|Default|GetDeltaTMax))))
  (Variables|Default|SetYVelocity (|((Dy-(((0.500000*g)*t)*t))/t) 0.0 (Variables|/Game/Blueprints/BP_Planet.BP_Planet_C|GetGravity (Variables|Default|GetNearestPlanet)) (* (/ (Math|Vector|Distance(Vector) (Transformation|GetActorLocation) (Variables|Default|GetEndPoint)) (Variables|Default|GetDistanceMax)) (Variables|Default|GetDeltaTMax)))))

(event EventTick
  (params (DeltaSeconds :type Float%20%28single-precision%29))
  (bind _projectile (Variables|Default|GetProjectile))
  (bind _nearestplanet (Variables|Default|GetNearestPlanet))
  (bind _relativelocation (Variables|/Script/Engine.SceneComponent|GetRelativeLocation _projectile))
  (bind _gravity (Variables|/Game/Blueprints/BP_Planet.BP_Planet_C|GetGravity _nearestplanet))
  (Transformation|SetRelativeLocation _projectile (Math|Vector|MakeVector (|(x0+(v0x*Dt)) (.x _relativelocation) (Variables|Default|GetXVelocity) DeltaSeconds) (|((y0+(V0y*t))+((0.500000*g)*(t*t))) (.y _relativelocation) (* (Variables|Default|GetYVelocity) -1.0) DeltaSeconds _gravity) 0.0) false false)
  (Variables|Default|SetYVelocity (+ (Variables|Default|GetYVelocity) (* _gravity DeltaSeconds))))

(fn ConstructionScript)