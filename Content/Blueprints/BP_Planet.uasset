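; BP_Planet is a possessable planet with a spring arm that serves as a rotatable view around it.
; The planet flagged as the start planet has the first player controller possess it on BeginPlay.
; While the CamMovementInput axis reads exactly 1, move-right and move-forward values rotate the arm's pitch and yaw.
; The construction script scales arm length with the planet's X scale.
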(event EventBeginPlay
  (if (Variables|Default|GetisStartPlanet)
    (Pawn|Possess (Game|GetPlayerController 0) self)))

(event Input|AxisEvents|InputAxisCamMovementInput
  (params (AxisValue :type Float%20%28single-precision%29))
  (if (== AxisValue 1.0)
    (Transformation|AddRelativeRotation (Variables|Default|GetSpringArm) (Math|Rotator|MakeRotator 0.0 (Input|AxisValues|GetMoveRight) (Input|AxisValues|GetMoveForward)) false false)))

(fn ConstructionScript
  (Variables|/Script/Engine.SpringArmComponent|SetTargetArmLength (Variables|Default|GetSpringArm) (* (.x (Transformation|GetActorScale3D)) (Variables|Default|GetStartSpringArmLength))))