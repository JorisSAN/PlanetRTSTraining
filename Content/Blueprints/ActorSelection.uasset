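; Selection volume actor that marks AI actors as selected when they overlap its Cube component.
; On BeginPlay it registers itself as the PlanetController's ActorSelection and prints a debug string.
; Overlap begin and end send IsInSelectionMessage through AI_Interface to implementing actors.
; Entering always selects, while leaving deselects only if the controller's PlanetClicked flag is true.
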(event OnComponentBeginOverlap(Cube)
  (params (OverlappedComponent :type Primitive%20Component%20Object%20Reference) (OtherActor :type Actor%20Object%20Reference) (OtherComp :type Primitive%20Component%20Object%20Reference) (OtherBodyIndex :type Integer) (bFromSweep :type Boolean) (SweepResult :type Hit%20Result%20Structure%20%28by%20ref%29))
  (if (Utilities|DoesObjectImplementInterface OtherActor "/Game/Blueprints/AI/AI_Interface.AI_Interface_C")
    (Class|AIInterface|IsinSelection(Message) OtherActor true)))

(event OnComponentEndOverlap(Cube)
  (params (OverlappedComponent :type Primitive%20Component%20Object%20Reference) (OtherActor :type Actor%20Object%20Reference) (OtherComp :type Primitive%20Component%20Object%20Reference) (OtherBodyIndex :type Integer))
  (if (Utilities|DoesObjectImplementInterface OtherActor "/Game/Blueprints/AI/AI_Interface.AI_Interface_C")
    (if (Variables|/Game/Blueprints/PlanetController.PlanetController_C|GetPlanetClicked (.AsPlanet%20Controller (Utilities|Casting|CastToPlanetController (Game|GetPlayerController 0))))
      (Class|AIInterface|IsinSelection(Message) OtherActor false))))

(event EventBeginPlay
  (bind _asplanet_controller (Utilities|Casting|CastToPlanetController (Game|GetPlayerController 0)))
  (Variables|/Game/Blueprints/PlanetController.PlanetController_C|SetActorSelection _asplanet_controller self)
  (Development|PrintString "AAA"))

(event Collision|EventActorBeginOverlap
  (params (OtherActor :type Actor%20Object%20Reference)))

(event EventTick
  (params (DeltaSeconds :type Float%20%28single-precision%29)))

(fn ConstructionScript)